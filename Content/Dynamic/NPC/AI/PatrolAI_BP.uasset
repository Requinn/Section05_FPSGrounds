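; AI controller for patrolling NPCs that runs the GaurdBehaviour behavior tree on the PatrolData blackboard.
; On BeginPlay it seeds the FocusActor key with the player pawn.
; AI perception updates then set FocusActor to sensed actors without the "Enemy" tag, or clear it when sensing fails.
; A Pawn cast keeps controllers, such as those reported by jump-landing events, from becoming the focus.
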(event `self.ReceiveBeginPlay`
  (bind _blackboardcomponent (`self.UseBlackboard` "/Game/Dynamic/NPC/AI/PatrolData.PatrolData"))
  (`BlackboardComponent.SetValueAsObject` _blackboardcomponent (`self.FocusActor`) (`GameplayStatics.GetPlayerPawn` 0))
  (`self.RunBehaviorTree` "/Game/Dynamic/NPC/AI/GaurdBehaviour.GaurdBehaviour"))

(event `self.AIPerception.OnTargetPerceptionUpdated`
  (params (Actor :type "Actor Object Reference") (Stimulus :type "AIStimulus Structure"))
  (bind _focusactor (`self.FocusActor`))
  (if (`self.ActorHasTag` Actor "Enemy")
    _
    (elif (`.bSuccessfullySensed` (break `AIStimulus` Stimulus))
      (bind _blackboardcomponent (`self.UseBlackboard` "/Game/Dynamic/NPC/AI/PatrolData.PatrolData"))
      ;[1 1 1] Cast to a Pawn to avoid the AI from selecting the controller on a jump landing event
      (bind _aspawn (cast `Pawn` Actor))
      (`BlackboardComponent.SetValueAsObject` _blackboardcomponent _focusactor _aspawn)
      (else
        (`BlackboardComponent.ClearValue` _blackboardcomponent _focusactor)))))

(fn `UserConstructionScript`)