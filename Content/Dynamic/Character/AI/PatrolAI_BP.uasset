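; AI controller for a patrolling guard that runs the GaurdBehaviour behavior tree on the PatrolData blackboard.
; BeginPlay seeds the FocusActor key with the player pawn.
; Perception updates write sensed pawns without the Player tag to that key and clear it on lost stimulus.
; Tick switches the controlled character's Aiming and Shooting on whenever the controller has a valid focus actor.
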(event `self.ReceiveBeginPlay`
  (bind _blackboardcomponent (`self.UseBlackboard` "/Game/Dynamic/Character/AI/PatrolData.PatrolData"))
  (`BlackboardComponent.SetValueAsObject` _blackboardcomponent (`self.FocusActor`) (`GameplayStatics.GetPlayerPawn` 0))
  (`self.RunBehaviorTree` "/Game/Dynamic/Character/AI/GaurdBehaviour.GaurdBehaviour"))

(event `self.AIPerception.OnTargetPerceptionUpdated`
  (params (Actor :type "Actor Object Reference") (Stimulus :type "AIStimulus Structure"))
  (bind _focusactor (`self.FocusActor`))
  (if (`self.ActorHasTag` Actor "Player")
    _
    (elif (`.bSuccessfullySensed` (break `AIStimulus` Stimulus))
      (bind _blackboardcomponent (`self.UseBlackboard` "/Game/Dynamic/Character/AI/PatrolData.PatrolData"))
      ;[1 1 1] Cast to a Pawn to avoid the AI from selecting the controller on a jump landing event
      (bind _aspawn (cast `Pawn` Actor))
      (`BlackboardComponent.SetValueAsObject` _blackboardcomponent _focusactor _aspawn)
      (else
        (`BlackboardComponent.ClearValue` _blackboardcomponent _focusactor)))))

(event `self.ReceiveTick`
  (params (DeltaSeconds :type "Float (single-precision)"))
  (bind _returnvalue (`KismetSystemLibrary.IsValid` (`self.GetFocusActor`)))
  (bind _ascharacter (cast `/Game/Dynamic/Character/Blueprint/Character` (`self.K2_GetPawn`)))
  (set `/Game/Dynamic/Character/Blueprint/Character.Aiming` _returnvalue _ascharacter)
  (set `/Game/Dynamic/Character/Blueprint/Character.Shooting` _returnvalue _ascharacter))

(fn `UserConstructionScript`)